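; BP_WaveLike is a procedural mesh Blueprint that defines a wave-like parametric surface.
; It overrides ParametricSurfaceFunction to map T and K to X and Y, with Z as a radial sine wave of the distance from the origin.
; The W variable divides that distance to set the wavelength, and an exponential of distance times Exp scales the amplitude.
; The construction script only calls its parent, and the event graph has no active logic.
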(event EventBeginPlay
  (|CallParentFunction) ; This node is disabled and will not be called.\nDrag off pins to build functionality.
)

(event Collision|EventActorBeginOverlap
  (params (OtherActor :type Actor%20Object%20Reference))
  (|CallParentFunction OtherActor) ; This node is disabled and will not be called.\nDrag off pins to build functionality.
)

(event EventTick
  (params (DeltaSeconds :type Float%20%28single-precision%29))
  (|CallParentFunction DeltaSeconds) ; This node is disabled and will not be called.\nDrag off pins to build functionality.
)

(fn ConstructionScript
  (|CallParentFunction))

(fn ParametricSurfaceFunction
  (params (t :type Float%20%28single-precision%29) (k :type Float%20%28single-precision%29))
  (bind _returnvalue (Math|Float|Square t))
  (bind _returnvalue_2 (Math|Float|Square k))
  (bind _returnvalue_3 (+ _returnvalue _returnvalue_2))
  (bind _returnvalue_4 (Math|Float|Sqrt _returnvalue_3))
  (return (Math|Vector|MakeVector t k (* (Math|Trig|Sin(Radians) (/ _returnvalue_4 (Variables|Default|Getw))) (Class|KismetMathLibrary|Exp (* _returnvalue_4 (Variables|Default|Getexp)))))))