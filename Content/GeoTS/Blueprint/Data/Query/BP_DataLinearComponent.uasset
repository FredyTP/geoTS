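; BP_DataLinearComponent is a data-driven component that slides the scene component it is attached to along a straight line according to a data value.
; On each data update, it reads the value for its Variable from the DataManager and normalizes it between MinValue and MaxValue, clamped to 0–1.
; That alpha interpolates between MinPosition and MaxPosition to set the parent's relative location, without sweep or Tick logic.
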(event EventBeginPlay)

(event EventTick
  (params (DeltaSeconds :type Float%20%28single-precision%29)))

(event EventOnDataUpdated
  (bind _minvalue (Variables|Default|GetMinValue))
  (Transformation|SetRelativeLocation (Transformation|GetAttachParent) (Math|Vector|Lerp(Vector) (Variables|Default|GetMinPosition) (Variables|Default|GetMaxPosition) (Math|Float|Clamp(Float) (Math|Float|SafeDivide (- (.value (Class|DataManager|GetEnum (Variables|Default|Get_dataManager) (Variables|Default|GetVariable))) _minvalue) (- (Variables|Default|GetMaxValue) _minvalue)))) false false))