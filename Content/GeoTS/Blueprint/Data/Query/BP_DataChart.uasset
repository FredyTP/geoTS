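; Data chart Blueprint that plots a selected DataManager variable against elapsed time on a Chart widget.
; Tick accumulates time, and each OnDataUpdated event adds a time/value point to the widget's SimpleTimeSeriesPlot.
; Series getter functions describe a single "Time" series backed by DataPoints, though the event graph never fills that array and pushes points directly to the plot.
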(event Collision|EventActorBeginOverlap
  (params (OtherActor :type Actor%20Object%20Reference)))

(event EventTick
  (params (DeltaSeconds :type Float%20%28single-precision%29))
  (Variables|Default|SetTime (+ DeltaSeconds (Variables|Default|GetTime))))

(event EventOnDataUpdated
  (bind _aschart (Utilities|Casting|CastToChart (UserInterface|GetUserWidgetObject (Variables|Default|GetWidget))))
  (Class|SimpleTimeSeriesPlot|AddDatapoint (Variables|/Game/GeoTS/Blueprint/Data/Query/UI/Chart.Chart_C|GetSimpleTimeSeriesPlot_66 _aschart) (Variables|/Game/GeoTS/Blueprint/Data/Query/UI/Chart.Chart_C|GetTimeId _aschart) (Math|Vector2D|MakeVector2D (Variables|Default|GetTime) (.value (Class|DataManager|GetEnum (Variables|Default|Get_dataManager) (Variables|Default|GetVariable))))))

(fn ConstructionScript)

(fn GetNumSeries
  (return 1))

(fn GetSeriesDatapoints
  (params (SeriesIdx :type Integer))
  (return (Variables|Default|GetDataPoints)))

(fn GetSeriesId
  (params (CatIdx :type Integer))
  (return "Time"))

(fn GetSeriesName
  (params (SeriesIdx :type Integer))
  (return "Time"))