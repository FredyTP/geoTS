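; Actor that displays one data variable from the DataManager on a widget screen.
; On OnDataUpdated it looks up the entry selected by Variable and casts the widget component's user widget to DataShow.
; It then writes the entry's name to VarName and its formatted value with unit suffix to VarValue.
; BeginPlay, Tick, overlap, the construction script and NewFunction0 do nothing.
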(event EventBeginPlay)

(event Collision|EventActorBeginOverlap
  (params (OtherActor :type Actor%20Object%20Reference)))

(event EventTick
  (params (DeltaSeconds :type Float%20%28single-precision%29)))

(event EventOnDataUpdated
  (bind _variable (Variables|Default|GetVariable))
  (bind __datamanager (Variables|Default|Get_dataManager))
  (bind _returnvalue (Class|DataManager|GetEnum __datamanager _variable))
  (bind _asdata_show (Utilities|Casting|CastToDataShow (UserInterface|GetUserWidgetObject (Variables|Default|GetWidget))))
  (Rendering|Components|TextRender|SetText (Variables|/Game/GeoTS/Blueprint/Data/Query/UI/DataShow.DataShow_C|GetVarName _asdata_show) (Utilities|Text|ToText(String) (.name _returnvalue)))
  (Rendering|Components|TextRender|SetText (Variables|/Game/GeoTS/Blueprint/Data/Query/UI/DataShow.DataShow_C|GetVarValue _asdata_show) (Utilities|Text|ToText(String) (Utilities|String|Append (Utilities|String|ToString(Text) (Utilities|Text|ToText(Float) (.value _returnvalue) "HalfFromZero")) (.unit _returnvalue)))))

(fn ConstructionScript)

(fn NewFunction0
  (params (InFloat :type Float%20%28single-precision%29)))