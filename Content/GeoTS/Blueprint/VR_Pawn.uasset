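; VR player pawn that draws on BP_Whiteboard actors with the right motion controller and clicks widgets.
; While the right trigger is fully pulled, short angled traces from the controller find the board's collision UV, setting its LastPoint and feeding DrawOnWhiteboard on Tick.
; The right trackpad acts as a left mouse button through WidgetInteraction.
; On BeginPlay, a SteamVR headset switches the tracking origin to floor level.
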(event EventTick
  (params (DeltaSeconds :type Float%20%28single-precision%29))
  (bind _returnvalue (Math|Vector|RotatorfromAxisandAngle "1.000000,0.000000, 0" -5e+01))
  (bind _motioncontroller_r (Variables|Default|GetMotionController_R))
  (bind _returnvalue_2 (Transformation|GetWorldLocation _motioncontroller_r))
  (bind _returnvalue_3 (Math|Vector|GetForwardVector _motioncontroller_r))
  (bind _returnvalue_4 (Math|Vector|RotateVector _returnvalue_3 _returnvalue))
  ;[1 1 1] Whiteboard Logic
  (if (Variables|Default|GetbIsDrawing)
    (bind (_outhit _returnvalue_5) (Collision|LineTraceByChannel (- _returnvalue_2 (* _returnvalue_4 5.0)) (+ _returnvalue_2 (* _returnvalue_4 20)) "TraceTypeQuery1" true 0 "None"))
    (if _returnvalue_5
      (Development|PrintString "colision")
      (bind _asbp_whiteboard (Utilities|Casting|CastToBP_Whiteboard (.HitActor (Collision|BreakHitResult _outhit))))
      (Default|DrawonWhiteboard _asbp_whiteboard (.UV (Class|GameplayStatics|FindCollisionUV _outhit)))
      (Development|PrintString "drawed!!"))))

(event Collision|EventActorBeginOverlap
  (params (OtherActor :type Actor%20Object%20Reference)))

(event EventBeginPlay
  (bind _returnvalue (Class|HeadMountedDisplayFunctionLibrary|GetHMDDeviceName))
  ;[1 1 1] Switch origin height
  (Development|PrintString (Utilities|String|ToString(Name) _returnvalue) true true "(R=0.000000,G=0.660000,B=1.000000,A=1.000000)" 1e+01)
  (switch name _returnvalue
    (:Steam%20VR
      (Class|HeadMountedDisplayFunctionLibrary|SetTrackingOrigin "Floor"))))

(event Input|ActionEvents|InputActionMotionControllerRTrackpad
  (params (Key :type Key%20Structure :default "None"))
  (bind _widgetinteraction (Variables|Default|GetWidgetInteraction))
  (:Pressed
    (Class|WidgetInteractionComponent|PressPointerKey _widgetinteraction "LeftMouseButton"))
  (:Released
    (Class|WidgetInteractionComponent|ReleasePointerKey _widgetinteraction "LeftMouseButton")))

(event Input|AxisEvents|InputAxisMotionControllerRTrigger
  (params (AxisValue :type Float%20%28single-precision%29))
  (bind _returnvalue (Math|Vector|RotatorfromAxisandAngle "1.000000,0.000000, 0" -5e+01))
  (bind _motioncontroller_r (Variables|Default|GetMotionController_R))
  (bind _returnvalue_2 (Transformation|GetWorldLocation _motioncontroller_r))
  (bind _returnvalue_3 (Math|Vector|GetForwardVector _motioncontroller_r))
  (bind _returnvalue_4 (Math|Vector|RotateVector _returnvalue_3 _returnvalue))
  ;[1 1 1] Whiteboard Logic
  (if (> AxisValue 0.99)
    (Variables|Default|SetbIsDrawing true)
    (bind (_outhit _returnvalue_5) (Collision|LineTraceByChannel (- _returnvalue_2 (* _returnvalue_4 5.0)) (+ _returnvalue_2 (* _returnvalue_4 20)) "TraceTypeQuery1" true 0 "None"))
    (if _returnvalue_5
      (bind _asbp_whiteboard (Utilities|Casting|CastToBP_Whiteboard (.HitActor (Collision|BreakHitResult _outhit))))
      (Variables|/Game/GeoTS/Blueprint/Whiteboard/BP_Whiteboard.BP_Whiteboard_C|SetlastPoint _asbp_whiteboard (.UV (Class|GameplayStatics|FindCollisionUV _outhit))))
    (else
      (Variables|Default|SetbIsDrawing false))))

(fn ConstructionScript)