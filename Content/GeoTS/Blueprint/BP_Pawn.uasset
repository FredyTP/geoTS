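; Player pawn that walks, looks around, zooms via mouse-wheel FOV and draws on BP_Whiteboard actors.
; Holding right mouse locks look input and line-traces from the cursor each tick, passing the hit's collision UV to the whiteboard's draw function.
; The initial press seeds the board's last point to start a stroke.
; Left mouse drives a WidgetInteraction pointer, and the ClearWhiteboard input wipes every board in the level.
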(event EventTick
  (params (DeltaSeconds :type Float%20%28single-precision%29))
  (bind _returnvalue (Game|GetPlayerController 0))
  (bind (_worldlocation _worlddirection) (Game|Player|ConvertMouseLocationToWorldSpace _returnvalue))
  ;[1 1 1] Whiteboard Logic
  (if (Variables|Default|GetbIsDrawing)
    (bind (_outhit _returnvalue_2) (Collision|LineTraceByChannel _worldlocation (+ _worldlocation (* _worlddirection 5e+02)) "TraceTypeQuery1" true 0 "None"))
    (if _returnvalue_2
      (bind _asbp_whiteboard (Utilities|Casting|CastToBP_Whiteboard (.HitActor (Collision|BreakHitResult _outhit))))
      (Default|DrawonWhiteboard _asbp_whiteboard (.UV (Class|GameplayStatics|FindCollisionUV _outhit))))))

(event Collision|EventActorBeginOverlap
  (params (OtherActor :type Actor%20Object%20Reference)))

(event Input|ActionEvents|InputActionClearWhiteboard
  (params (Key :type Key%20Structure :default "None"))
  ;[1 1 1] Clear Whiteboard
  (:Pressed
    (bind _outactors (Actor|GetAllActorsOfClass "/Game/GeoTS/Blueprint/Whiteboard/BP_Whiteboard.BP_Whiteboard_C"))
    (for _array_element _outactors
      (Default|ClearWhiteboard _array_element))))

(event Input|AxisEvents|InputAxisWalkForward
  (params (AxisValue :type Float%20%28single-precision%29))
  ;[1 1 1] Walk Input
  (Pawn|Input|AddMovementInput (Math|Vector|GetForwardVector (Pawn|GetControlRotation :!class /Script/Engine.Pawn)) AxisValue false))

(event Input|AxisEvents|InputAxisWalkRight
  (params (AxisValue :type Float%20%28single-precision%29))
  ;[1 1 1] Walk Input
  (Pawn|Input|AddMovementInput (Math|Vector|GetRightVector (Pawn|GetControlRotation :!class /Script/Engine.Pawn)) AxisValue false))

(event Input|AxisEvents|InputAxisTurn
  (params (AxisValue :type Float%20%28single-precision%29))
  ;[1 1 1] RotationControl
  (if (not (Variables|Default|GetbIsDrawing))
    (Pawn|Input|AddControllerYawInput (* AxisValue (Variables|Default|GetAxisTurnRate)))))

(event Input|AxisEvents|InputAxisLookUp
  (params (AxisValue :type Float%20%28single-precision%29))
  ;[1 1 1] RotationControl
  (if (not (Variables|Default|GetbIsDrawing))
    (Pawn|Input|AddControllerPitchInput (* AxisValue (Variables|Default|GetAxisLookUpRate)))))

(event Input|MouseEvents|MouseWheelAxis
  (params (AxisValue :type Float%20%28single-precision%29))
  ;[1 1 1] FielOfView Control
  (bind _output_get (Variables|Default|SetFieldOfView (+ (* AxisValue (Variables|Default|GetFOV_Scale)) (Variables|Default|GetFieldOfView))))
  (Camera|SetFieldOfView (Variables|Default|GetCamera) _output_get))

(event Input|MouseEvents|LeftMouseButton
  (params (Key :type Key%20Structure :default "None"))
  (:Pressed
    (Class|WidgetInteractionComponent|PressPointerKey (Variables|Default|GetWidgetInteraction) "LeftMouseButton"))
  (:Released
    (Class|WidgetInteractionComponent|ReleasePointerKey (Variables|Default|GetWidgetInteraction) "LeftMouseButton")))

(event Input|MouseEvents|RightMouseButton
  (params (Key :type Key%20Structure :default "None"))
  (bind _returnvalue (Game|GetPlayerController 0))
  (bind (_worldlocation _worlddirection) (Game|Player|ConvertMouseLocationToWorldSpace _returnvalue))
  ;[1 1 1] Whiteboard Logic
  (:Pressed
    (Variables|Default|SetbIsDrawing true)
    (bind (_outhit _returnvalue_2) (Collision|LineTraceByChannel _worldlocation (+ _worldlocation (* _worlddirection 5e+02)) "TraceTypeQuery1" true 0 "None"))
    (if _returnvalue_2
      (bind _asbp_whiteboard (Utilities|Casting|CastToBP_Whiteboard (.HitActor (Collision|BreakHitResult _outhit))))
      (Variables|/Game/GeoTS/Blueprint/Whiteboard/BP_Whiteboard.BP_Whiteboard_C|SetlastPoint _asbp_whiteboard (.UV (Class|GameplayStatics|FindCollisionUV _outhit)))))
  (:Released
    (Variables|Default|SetbIsDrawing false)))

(fn ConstructionScript)