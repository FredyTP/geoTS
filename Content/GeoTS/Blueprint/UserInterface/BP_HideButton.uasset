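; BP_HideButton is an actor whose widget component shows a HideButton, labelled "Esconder" (Hide) plus its collection name.
; On BeginPlay it passes Collection to the widget, sets the label, enables input from player controller 0 and shows the button.
; The ShowGUI input drives a FlipFlop into SetWidgetVisibility, which switches both widget visibility and collision between query-only and none.
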(event EventBeginPlay
  (bind _ashide_button (Utilities|Casting|CastToHideButton (UserInterface|GetUserWidgetObject (Variables|Default|GetWidget))))
  (Variables|/Game/GeoTS/Blueprint/UserInterface/HideButton.HideButton_C|SetCollectionName _ashide_button (Variables|Default|GetCollection))
  (Rendering|Components|TextRender|SetText (Variables|/Game/GeoTS/Blueprint/UserInterface/HideButton.HideButton_C|GetTextButton _ashide_button) (Utilities|Text|ToText(String) (Utilities|String|Append "Esconder" (Variables|/Game/GeoTS/Blueprint/UserInterface/HideButton.HideButton_C|GetCollectionName _ashide_button))))
  (Input|EnableInput (Game|GetPlayerController 0))
  (CallFunction|SetWidgetVisibility true))

(event Input|ActionEvents|InputActionShowGUI
  (params (Key :type Key%20Structure :default "None"))
  (:Pressed
    (bind _isa (Utilities|FlowControl|FlipFlop)
      (:A
        _)
      (:B
        _))
    (CallFunction|SetWidgetVisibility _isa)))

(fn ConstructionScript)

(fn SetWidgetVisibility
  (params (bVisible :type Boolean))
  (bind _widget (Variables|Default|GetWidget))
  (bind _widget_2 (Variables|Default|GetWidget))
  (bind _returnvalue (UserInterface|GetUserWidgetObject _widget))
  (if bVisible
    (Widget|SetVisibility _returnvalue "Visible")
    (Collision|SetCollisionEnabled _widget_2 "QueryOnly")
    (else
      (Widget|SetVisibility _returnvalue "Hidden")
      (Collision|SetCollisionEnabled _widget_2 "NoCollision"))))