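; TriggerBox_Blueprint is a trigger volume that shows or hides whiteboard UI as actors enter and leave it.
; Begin and end overlap each fetch every BP_WhiteboardUI actor, toggle its Widget's visibility with propagation to children, and print a debug string.
; The VR_Pawn casts are not wired to the overlap events, so any overlapping actor triggers the toggle.
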(event EventBeginPlay)

(event Collision|EventActorBeginOverlap
  (params (OtherActor :type Actor%20Object%20Reference))
  (bind _outactors (Actor|GetAllActorsOfClass "/Game/GeoTS/Blueprint/UserInterface/BP_WhiteboardUI.BP_WhiteboardUI_C"))
  (for _array_element _outactors
    (Rendering|SetVisibility (Variables|/Game/GeoTS/Blueprint/UserInterface/BP_WhiteboardUI.BP_WhiteboardUI_C|GetWidget _array_element) true true))
  (Development|PrintString "show"))

(event EventTick
  (params (DeltaSeconds :type Float%20%28single-precision%29)))

(event Collision|EventActorEndOverlap
  (params (OtherActor :type Actor%20Object%20Reference))
  (bind _outactors (Actor|GetAllActorsOfClass "/Game/GeoTS/Blueprint/UserInterface/BP_WhiteboardUI.BP_WhiteboardUI_C"))
  (for _array_element _outactors
    (Rendering|SetVisibility (Variables|/Game/GeoTS/Blueprint/UserInterface/BP_WhiteboardUI.BP_WhiteboardUI_C|GetWidget _array_element) false true))
  (Development|PrintString "HIDE"))

(fn ConstructionScript)