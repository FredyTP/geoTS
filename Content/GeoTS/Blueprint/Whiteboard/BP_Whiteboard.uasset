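; Whiteboard actor that draws marker strokes into the RT_Whiteboard render target from UV positions passed to DrawOnWhiteboard.
; On BeginPlay it creates a dynamic marker material sized by MarkerSize.
; DrawLine fills gaps since the stored LastPoint with interpolated stamps spaced by Treshold and capped by MaxPointsLine, then saves the new point.
; DrawPoint stamps by rendering the material at that location; ClearWhiteboard clears the target to opaque black.
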(event Custom|DrawOnWhiteboard
  (params (DrawPosition :type Vector%202D%20Structure))
  (CallFunction|DrawLine DrawPosition (Variables|Default|GetlastPoint)))

(event EventBeginPlay
  (bind _returnvalue (Rendering|Material|CreateDynamicMaterialInstance "/Game/GeoTS/Blueprint/Whiteboard/M_WhiteboarMarker.M_WhiteboarMarker" "None" :!class /Script/Engine.KismetMaterialLibrary))
  (Variables|Default|SetWhiteboardMarker_MI _returnvalue)
  (Rendering|Material|SetScalarParameterValue (Variables|Default|GetWhiteboardMarker_MI) "DrawSize" (Variables|Default|GetMarkerSize) :!class /Script/Engine.MaterialInstanceDynamic))

(event Collision|EventActorBeginOverlap
  (params (OtherActor :type Actor%20Object%20Reference)))

(event EventTick
  (params (DeltaSeconds :type Float%20%28single-precision%29)))

(fn ConstructionScript)

(fn DrawPoint
  (params (PointUV :type Vector%202D%20Structure))
  (bind _whiteboardmarker_mi (Variables|Default|GetWhiteboardMarker_MI))
  (Rendering|Material|SetVectorParameterValue _whiteboardmarker_mi "DrawLocation" (Math|Conversions|ToLinearColor(Vector) (Math|Conversions|ToVector(Vector2D) PointUV)) :!class /Script/Engine.MaterialInstanceDynamic)
  (Rendering|DrawMaterialtoRenderTarget "/Game/GeoTS/Blueprint/Whiteboard/RT_Whiteboard.RT_Whiteboard" _whiteboardmarker_mi))

(fn DrawLine
  (params (PointUV :type Vector%202D%20Structure) (LastPointUV :type Vector%202D%20Structure))
  (bind _returnvalue (Class|KismetMathLibrary|GetAbs2D PointUV))
  (LocalVariables|SetContador 1)
  (LocalVariables|SetlocalPoint _returnvalue)
  (LocalVariables|SetlocalLastPoint LastPointUV)
  (while (and (< (LocalVariables|GetContador) (Math|Float|Round (Math|Float|SafeDivide (Math|Vector|Distance2D(Vector) (LocalVariables|GetlocalLastPoint) (LocalVariables|GetlocalPoint)) (Variables|Default|GetTreshold)))) (< (LocalVariables|GetContador) (Variables|Default|GetMaxPointsLine)))
    (CallFunction|DrawPoint (+ (* (/ (- (LocalVariables|GetlocalPoint) (LocalVariables|GetlocalLastPoint)) (Math|Conversions|ToFloat(Integer) (Math|Float|Round (Math|Float|SafeDivide (Math|Vector|Distance2D(Vector) (LocalVariables|GetlocalLastPoint) (LocalVariables|GetlocalPoint)) (Variables|Default|GetTreshold))))) (Math|Conversions|ToFloat(Integer) (LocalVariables|GetContador))) (LocalVariables|GetlocalLastPoint)))
    (LocalVariables|SetContador (+ (LocalVariables|GetContador) 1)))
  (CallFunction|DrawPoint _returnvalue)
  (Variables|Default|SetlastPoint _returnvalue))

(fn ClearWhiteboard
  (Rendering|ClearRenderTarget2D "/Game/GeoTS/Blueprint/Whiteboard/RT_Whiteboard.RT_Whiteboard"))